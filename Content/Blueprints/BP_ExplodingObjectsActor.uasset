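; A replicated exploding actor that detonates on a timer a few seconds after BeginPlay.
; The server alone runs the timer, then calls a multicast that fires a radial force impulse, hides the actor and disables its collision on all clients.
; A short lifespan set after the multicast handles delayed removal; the DestroyActor node is left unconnected.
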(event `self.ReceiveBeginPlay`
  (if (`self.HasAuthority`)
    (`KismetSystemLibrary.K2_SetTimerDelegate` (delegate `Explode`) 4.0)))

(event `Explode`
  ;[1 1 1] server上触发
  ;[1 1 1] 通知给所有客户端
  (`self.MulticastExplode`)
  (`self.SetLifeSpan` 2.0))

(event `MulticastExplode`
  ;[1 1 1] 网络复制多播
  (`RadialForceComponent.FireImpulse` (`self.RadialForce`))
  (`self.SetActorHiddenInGame` true)
  (`self.SetActorEnableCollision` false))

(fn `UserConstructionScript`)