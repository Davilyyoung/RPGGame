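; Interactable save point actor that lights a fire and saves the game when used.
; Interact sets FireActive before writing the save through SSaveGameSubsystem, then refreshes the flames.
; OnActorLoaded runs the same UpdateFlames, which activates the particle system only if FireActive is true and never turns it off.
; Both paths print debug strings, and the interact text is empty.
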(event `SGamePlayInterface.Interact`
  (params (InstigatorPawn :type "Pawn Object Reference"))
  (set `self.bFireActive` true)
  (`SSaveGameSubsystem.WriteSaveGame` (subsystem `SSaveGameSubsystem`))
  (`KismetSystemLibrary.PrintString` "SaveGame")
  (`self.UpdateFlames`))

(event `SGamePlayInterface.OnActorLoaded`
  (`self.UpdateFlames`)
  (`KismetSystemLibrary.PrintString` "LoadGame"))

(event `UpdateFlames`
  (if (`self.bFireActive`)
    (`ActorComponent.Activate` (`self.ParticleSystem`) false)))

(fn `GetInteractText`
  (params (InstigatorPawn :type "Pawn Object Reference"))
  (returns (ReturnValue :type Text))
  (return ""))

(fn `UserConstructionScript`)