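; BP_ApplyEff is a trigger volume that grants a configurable action effect to actors that overlap it.
; On the server, the box overlap looks up the other actor's SActionComponent and, if valid, adds EffectActionToApply with the trigger as instigator.
; The construction script sets the text render and billboard sprite from variables to label each placed instance.
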(event `self.Box.OnComponentBeginOverlap`
  (params (OverlappedComponent :type "PrimitiveComponent Object Reference") (OtherActor :type "Actor Object Reference") (OtherComp :type "PrimitiveComponent Object Reference") (OtherBodyIndex :type Integer) (bFromSweep :type Boolean) (SweepResult :type "HitResult Structure (by ref)"))
  (bind _returnvalue (`self.GetComponentByClass` OtherActor "/Script/RPGGame.SActionComponent"))
  (`/Engine/EditorBlueprintResources/ActorMacros.Switch Has Authority`
    (:`Authority`
      (`/Engine/EditorBlueprintResources/StandardMacros.IsValid` _returnvalue
        (:`Is Valid`
          (`SActionComponent.AddAction` _returnvalue self (`self.Effect Action to Apply`)))))))

(fn `UserConstructionScript`
  (`TextRenderComponent.K2_SetText` (`self.TextRender`) (`self.Text`))
  (`BillboardComponent.SetSprite` (`self.Billboard`) (`self.BiliboardSprite`)))