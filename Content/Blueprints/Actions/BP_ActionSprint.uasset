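; Sprint action Blueprint that raises a character's walk speed while the action runs.
; On start, it calls the parent action logic, then adds a bonus speed to the instigator's CharacterMovementComponent MaxWalkSpeed.
; On stop, it calls the parent logic and subtracts the same bonus, a relative change rather than restoring a saved value.
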(event `self.StartAction`
  (params (Instigator :type "Actor Object Reference"))
  (bind _returnvalue (`Actor.GetComponentByClass` Instigator "/Script/Engine.CharacterMovementComponent"))
  (`parent.StartAction` Instigator)
  (`/Engine/EditorBlueprintResources/StandardMacros.IsValid` _returnvalue
    (:`Is Valid`
      (set `CharacterMovementComponent.MaxWalkSpeed` (+ (`CharacterMovementComponent.MaxWalkSpeed` _returnvalue) (`self.BounsSpeed`)) _returnvalue))))

(event `self.StopAction`
  (params (Instigator :type "Actor Object Reference"))
  (bind _returnvalue (`Actor.GetComponentByClass` Instigator "/Script/Engine.CharacterMovementComponent"))
  (`parent.StopAction` Instigator)
  (`/Engine/EditorBlueprintResources/StandardMacros.IsValid` _returnvalue
    (:`Is Valid`
      (set `CharacterMovementComponent.MaxWalkSpeed` (- (`CharacterMovementComponent.MaxWalkSpeed` _returnvalue) (`self.BounsSpeed`)) _returnvalue))))