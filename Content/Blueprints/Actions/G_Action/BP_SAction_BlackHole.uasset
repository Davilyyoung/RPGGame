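; BP_SAction_BlackHole is the Black Hole action, gated by and paid for with the instigator's Rage attribute.
; CanStart extends the parent check, requiring Rage of at least RageCost and printing "Not Enough Rage" when short.
; StartAction applies RageCost as a negative Rage delta through the attributes component, then defers to the parent StartAction for the rest of the behavior.
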(event `self.StartAction`
  (params (Instigator :type "Actor Object Reference"))
  ;[1 1 1] 加愤怒
  (bind _returnvalue (`SAttributeComponent.GetAttributes` Instigator))
  (`SAttributeComponent.ApplyRage` _returnvalue Instigator (/ (`self.RageCost`) -1.0))
  (`parent.StartAction` Instigator))

(fn `CanStart`
  (params (Instigator :type "Actor Object Reference"))
  (returns (ReturnValue :type Boolean))
  (bind _returnvalue (`parent.CanStart` Instigator))
  (if _returnvalue
    (bind _returnvalue_2 (`SAttributeComponent.GetAttributes` Instigator))
    (if (>= (`SAttributeComponent.GetRage` _returnvalue_2) (`self.RageCost`))
      (return true)
      (else
        (`KismetSystemLibrary.PrintString` "Not Enough Rage")
        (return false)))
    (else
      (return false))))