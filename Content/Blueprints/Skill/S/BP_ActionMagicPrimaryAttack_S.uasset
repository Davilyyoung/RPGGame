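; Shinbi's magic primary attack action, which spawns a ring of wolf skill actors (BP_S_SKill) around the aimed point.
; On start, a camera line trace picks the hit location, or the trace's end point if nothing is hit.
; A custom delayed-loop macro staggers the spawns, stepping the angle each time and stopping the action within every iteration.
; WolfSkill offsets each actor by distance and height, yawed toward the center.
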(event `self.StartAction`
  (params (Instigator :type "Actor Object Reference"))
  (`parent.StartAction` Instigator)
  (bind _asbp_player_charecter_shinbi (cast `/Game/Blueprints/GameModeClass/BP_PlayerCharecter_Shinbi` Instigator))
  (bind _cameracomp (`SCharacter.CameraComp` _asbp_player_charecter_shinbi))
  (bind _returnvalue (+ (* (`SceneComponent.GetForwardVector` _cameracomp) 2000.0) (`SceneComponent.K2_GetComponentLocation` _cameracomp)))
  (bind (_outhit _returnvalue_2) (`KismetSystemLibrary.LineTraceSingleForObjects` (`SceneComponent.K2_GetComponentLocation` _cameracomp) _returnvalue (`|MakeArray` "ObjectTypeQuery1" "ObjectTypeQuery2" "ObjectTypeQuery3" "ObjectTypeQuery4" :!type "EObjectTypeQuery Enum"))) ; 射线检测
  (`self.SpawnWolf` (select `bool` _returnvalue_2 :`false` _returnvalue :`true` (`.Location` (`GameplayStatics.BreakHitResult` _outhit)))))

(event `SpawnWolf`
  (params (SpawnPoint :type "Vector Structure") (Instigator :type "Pawn Object Reference"))
  ;[1 1 1] LoopDelay
  (`self.ForLoopDelay` 1 (`self.WolfNum`) 0.1
    (:`LoopBody`
      (bind _output_get (set `self.Angle` (+ (`self.Angle`) (`self.AngleOffset`))))
      (`self.WolfSkill` (`self.Disrance`) _output_get (`self.Hight`) SpawnPoint Instigator)
      (`self.StopAction` Instigator))))

(event `self.StopAction`
  (params (Instigator :type "Actor Object Reference"))
  (`parent.StopAction` Instigator))

(fn `WolfSkill`
  (params (Distance :type "Float (double-precision)") (Angle :type "Float (double-precision)") (Height :type "Float (double-precision)") (SpawnLocation :type "Vector Structure") (Instigator :type "Pawn Object Reference"))
  (bind _returnvalue (`KismetMathLibrary.MakeVector` (+ (.x SpawnLocation) (* Distance (`KismetMathLibrary.DegSin` Angle))) (+ (.y SpawnLocation) (* Distance (`KismetMathLibrary.DegCos` Angle))) (+ (.z SpawnLocation) Height)))
  (bind (_returnvalue_roll _returnvalue_pitch _returnvalue_yaw) (`KismetMathLibrary.BreakRotator` (`KismetMathLibrary.MakeRotFromX` (- SpawnLocation _returnvalue))))
  (`|SpawnActorFromClass` "/Game/Blueprints/Skill/S/BP_S_SKill.BP_S_SKill_C" (`KismetMathLibrary.MakeTransform` _returnvalue (`KismetMathLibrary.MakeRotator` 0.0 0.0 _returnvalue_yaw)) "AlwaysSpawn" "OverrideRootScale" null Instigator))