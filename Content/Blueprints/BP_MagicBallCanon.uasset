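; BP_MagicBallCanon is an automatic turret actor that fires BP_MagicPrimaryAttack projectiles.
; A looping timer set on BeginPlay drives the firing, with AutoFire spawning each projectile at the actor's location and rotation.
; Each Tick turns the Arrow component to face the first player's pawn using a look-at rotation, while the spawn reads the actor's rotation rather than the Arrow's.
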(event `self.ReceiveBeginPlay`
  (`KismetSystemLibrary.K2_SetTimerDelegate` (`|CreateDelegate` :!event `AutoFire`) 2.0 true))

(event `AutoFire`
  (`|SpawnActorFromClass` "/Game/Blueprints/Skill/G/BP_MagicPrimaryAttack.BP_MagicPrimaryAttack_C" (`KismetMathLibrary.MakeTransform` (`self.K2_GetActorLocation`) (`self.K2_GetActorRotation`)) "Undefined" "OverrideRootScale" null null))

(event `self.ReceiveTick`
  (params (DeltaSeconds :type "Float (single-precision)"))
  (`SceneComponent.K2_SetWorldRotation` (`self.Arrow`) (`KismetMathLibrary.FindLookAtRotation` (`self.K2_GetActorLocation`) (`self.K2_GetActorLocation` (`GameplayStatics.GetPlayerPawn` 0))) false false))

(fn `UserConstructionScript`)