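; Blueprint treasure chest actor whose Interact event calls the parent implementation and prints a debug message.
; Two disconnected chains remain in the event graph and never run.
; One checks the SActionComponent's active gameplay tags for an exact RequiredKeyCard match and prints the missing tag.
; The other flip-flops a timeline that pitches LidMesh open or closed, activating a particle system when finished.
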(event `SGamePlayInterface.Interact`
  (params (InstigatorPawn :type "Pawn Object Reference"))
  (`parent.Interact` InstigatorPawn)
  (`KismetSystemLibrary.PrintString` "TreasureChest Interact(BP)"))

(fn `UserConstructionScript`)